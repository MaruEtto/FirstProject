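; BP_ActiveSphere is an actor that moves in a straight line and bounces off whatever blocks it, slowing and shrinking with each hit.
; Tick does a swept world offset along Direction, then on a blocking hit reflects it around the normal and reduces Speed and scale down to minimums.
; Both decrements are fixed tenths of the starting values, cached at BeginPlay.
; ScaleSphere and ChangeSpeed hold percentage-based variants that the event graph never calls.
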(event EventBeginPlay
  (Variables|Default|SetSlowing%20Down (* (Variables|Default|GetSpeed) 0.1))
  (Variables|Default|SetScale (* (Transformation|GetActorScale3D) "0.100000,0.100000,0.100000")))

(event EventTick
  (params (DeltaSeconds :type Float%20%28single-precision%29))
  (bind _sweephitresult (Transformation|AddActorWorldOffset (* (* (Variables|Default|GetDirection) (Variables|Default|GetSpeed)) DeltaSeconds) true))
  (if (.bBlockingHit (Collision|BreakHitResult _sweephitresult))
    (Variables|Default|SetDirection (Math|Vector|GetReflectionVector (Variables|Default|GetDirection) (.Normal (Collision|BreakHitResult _sweephitresult))))
    (bind _output_get (Variables|Default|SetSpeed (Math|Float|Max(Float) (- (Variables|Default|GetSpeed) (Variables|Default|GetSlowing%20Down)) (Variables|Default|GetMinSpeed))))
    (Transformation|SetActorScale3D (Math|Vector|VectorComponentMax (- (Transformation|GetActorScale3D) (Variables|Default|GetScale)) (Variables|Default|GetMinScale)))))

(fn ConstructionScript)

(fn ScaleSphere
  (Transformation|SetActorScale3D (Math|Vector|VectorComponentMax (- (Transformation|GetActorScale3D) (* (Transformation|GetActorScale3D) "0.100000,0.100000,0.100000")) (Variables|Default|GetMinScale))))

(fn ChangeSpeed
  (if (>= (- (Variables|Default|GetSpeed) (* (Variables|Default|GetSpeed) 0.1)) (Variables|Default|GetMinSpeed))
    (bind _output_get (Variables|Default|SetSpeed (- (Variables|Default|GetSpeed) (* (Variables|Default|GetSpeed) 0.1))))
    (Development|PrintString (Utilities|String|ToString(Float) _output_get) true true "(R=0.000000,G=0.660000,B=1.000000,A=1.000000)" 3e+01)))